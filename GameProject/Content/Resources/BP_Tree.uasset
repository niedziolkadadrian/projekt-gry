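; BP_Tree is a tree resource actor that can break into pickable wood logs.
; DestroyIntoLogsAfter starts a timer that calls DestroyIntoLogs, which hides and destroys the tree and spawns PickableItem actors set to Resource_WoodLog.
; Logs are stacked along the mesh's up vector, spaced by their bounds, with physics enabled and mass taken from item weight.
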(event EventBeginPlay)

(event Collision|EventActorBeginOverlap
  (params (OtherActor :type Actor%20Object%20Reference)))

(event EventTick
  (params (DeltaSeconds :type Float%20%28single-precision%29)))

(fn ConstructionScript)

(fn DestroyIntoLogsAfter
  (params (Time%20to%20destroy :type Float%20%28single-precision%29))
  (Utilities|Time|SetTimerbyFunctionName 0 "DestroyIntoLogs" Time%20to%20destroy))

(fn DestroyIntoLogs
  (bind _treemesh (Variables|Default|GetTreeMesh))
  (Variables|Default|SetLocation (Transformation|GetWorldLocation _treemesh))
  (Variables|Default|SetRotation (Transformation|GetWorldRotation _treemesh))
  (Rendering|SetActorHiddenInGame true)
  (Actor|DestroyActor)
  (for _index (range 0 2)
    (bind _returnvalue (Game|SpawnActorfromClass "/Script/GameProject.PickableItem" (Math|Transform|MakeTransform (Variables|Default|GetLocation) (Variables|Default|GetRotation)) "Undefined" 0 0))
    (Class|PickableItem|SetItem _returnvalue "/Game/Items/Resource_WoodLog.Resource_WoodLog_C")
    (Physics|SetSimulatePhysics (Variables|/Script/GameProject.PickableItem|GetMesh _returnvalue) true)
    (Class|PrimitiveComponent|SetMassOverrideinKg (Variables|/Script/GameProject.PickableItem|GetMesh _returnvalue) "None" (Variables|/Script/GameProject.ItemBase|GetWeight (Variables|/Script/GameProject.PickableItem|GetItem _returnvalue)) true)
    (Variables|Default|SetLocation (+ (Variables|Default|GetLocation) (* (Math|Vector|GetUpVector (Variables|Default|GetRotation)) (+ 2e+01 (.Z (Math|Vector|BreakVector (* (.BoxExtent (Collision|GetComponentBounds (Variables|/Script/GameProject.PickableItem|GetMesh _returnvalue))) 2.0)))))))))