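; Brimod ore spawner: a minable resource node that drops Brimod items and regrows after a random delay.
; MineBrimod clears the ore mesh and spawns physics-simulated PickableItems set to Resource_Brimod, offset sideways by their bounds and weighted by item weight.
; It then starts a timer within the min/max respawn range that calls SpawnBrimod to restore the ore mesh.
; The event graph is empty, so mining is triggered externally.
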(event EventBeginPlay)

(event Collision|EventActorBeginOverlap
  (params (OtherActor :type Actor%20Object%20Reference)))

(event EventTick
  (params (DeltaSeconds :type Float%20%28single-precision%29)))

(fn ConstructionScript)

(fn MineBrimod
  (bind _mesh (Variables|Default|GetMesh))
  (Variables|Default|SetLocation (+ (Transformation|GetWorldLocation _mesh) (* (Math|Vector|GetUpVector _mesh) 2e+01) (* (Math|Vector|GetRightVector _mesh) 2e+01) (* (Math|Vector|GetForwardVector _mesh) 2e+01)))
  (Variables|Default|SetRotation (Transformation|GetWorldRotation _mesh))
  (Components|StaticMesh|SetStaticMesh (Variables|Default|GetMesh) 0)
  (for _index (range 0 1)
    (bind _returnvalue (Game|SpawnActorfromClass "/Script/GameProject.PickableItem" (Math|Transform|MakeTransform (Variables|Default|GetLocation) (Variables|Default|GetRotation)) "Undefined" 0 0))
    (Class|PickableItem|SetItem _returnvalue "/Game/Items/Resource_Brimod.Resource_Brimod_C")
    (Physics|SetSimulatePhysics (Variables|/Script/GameProject.PickableItem|GetMesh _returnvalue) true)
    (Class|PrimitiveComponent|SetMassOverrideinKg (Variables|/Script/GameProject.PickableItem|GetMesh _returnvalue) "None" (Variables|/Script/GameProject.ItemBase|GetWeight (Variables|/Script/GameProject.PickableItem|GetItem _returnvalue)) true)
    (Variables|Default|SetLocation (- (Variables|Default|GetLocation) (* (Math|Vector|GetRightVector (Variables|Default|GetRotation)) (+ (* (.Y (Math|Vector|BreakVector (.BoxExtent (Collision|GetComponentBounds (Variables|/Script/GameProject.PickableItem|GetMesh _returnvalue))))) 2.0) 2e+01)))))
  (Utilities|Time|SetTimerbyFunctionName 0 "SpawnBrimod" (Math|Random|RandomFloatinRange (Variables|Default|GetMinTimeToRespawn) (Variables|Default|GetMaxTimeToRespawn))))

(fn SpawnBrimod
  (Components|StaticMesh|SetStaticMesh (Variables|Default|GetMesh) (Variables|Default|GetBrimodOreMesh)))