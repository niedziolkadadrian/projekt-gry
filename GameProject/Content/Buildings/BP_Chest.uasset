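; BP_Chest is an interactable storage chest that shows its inventory alongside the player's.
; Focus caches the player's InputStateMachine and the HUD and shows an "E" hint, which losing focus hides.
; Interacting toggles both inventory widgets and quick slots, updates HUD input mode, and on opening saves the prior player state before entering CraftInv.
; An inventory-updated delegate refreshes the chest widget whenever contents change.
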(event Custom|OnInventoryUpdated_Event_0
  (bind _ingamehud (Variables|Default|GetInGameHUD)
    (:then
      (bind _returnvalue (Class|InGameHUD|GetInventoryWidget _ingamehud))
      (Class|InventoryWidget|Update _returnvalue (Variables|Default|GetChestInventory)))
    (:else)))

(event EventBeginPlay
  (EventDispatchers|AssignOnInventoryUpdated (Variables|Default|GetChestInventory) (delegate Custom|OnInventoryUpdated_Event_0)))

(event Collision|EventActorBeginOverlap
  (params (OtherActor :type Actor%20Object%20Reference)))

(event EventTick
  (params (DeltaSeconds :type Float%20%28single-precision%29)))

(event EventOnInteract
  (params (Caller :type Actor%20Object%20Reference))
  (bind _playerstatemachine (Variables|Default|GetPlayerStateMachine))
  (bind _ingamehud (Variables|Default|GetInGameHUD))
  (Variables|Default|SetPlayerInventory (Actor|GetComponentbyClass Caller "/Script/GameProject.InventoryComponent"))
  (if (Math|Boolean|ORBoolean (Utilities|Enum|Equal(Enum) (Variables|/Script/GameProject.InputStateMachine|GetActState (Variables|Default|GetPlayerStateMachine)) "UI_CraftInv") (Utilities|Enum|Equal(Enum) (Variables|/Script/GameProject.InputStateMachine|GetActState (Variables|Default|GetPlayerStateMachine)) "Building") (Utilities|Enum|Equal(Enum) (Variables|/Script/GameProject.InputStateMachine|GetActState (Variables|Default|GetPlayerStateMachine)) "PlayerInput"))
    (if (Variables|Default|GetisInvOpen)
      (bind _result (Math|Integer|DecrementInt (Variables|/Script/GameProject.InGameHUD|GetActiveUIElems _ingamehud))
        (:%20%20
          (if (< _result 0)
            (Variables|/Script/GameProject.InGameHUD|SetActiveUIElems _ingamehud 0))
          (Class|InGameHUD|ChangeInputType (Variables|Default|GetInGameHUD))
          (bind _returnvalue (Class|InGameHUD|GetPlayerInventoryWidget (Variables|Default|GetInGameHUD)))
          (Class|PlayerInventoryWidget|HideInventory _returnvalue)
          (bind _returnvalue_2 (Class|InGameHUD|GetInventoryWidget (Variables|Default|GetInGameHUD)))
          (Class|InventoryWidget|HideInventory _returnvalue_2)
          (bind _returnvalue_3 (Class|InGameHUD|GetQuickSlotsWidget (Variables|Default|GetInGameHUD)))
          (Class|QuickSlotsWidget|ShowQuickSlots _returnvalue_3)
          (Variables|Default|SetisInvOpen false)))
      (else
        (Math|Integer|IncrementInt (Variables|/Script/GameProject.InGameHUD|GetActiveUIElems (Variables|Default|GetInGameHUD))
          (:%20%20
            (Class|InGameHUD|ChangeInputType (Variables|Default|GetInGameHUD))
            (bind _returnvalue_4 (Class|InGameHUD|GetQuickSlotsWidget (Variables|Default|GetInGameHUD)))
            (Class|QuickSlotsWidget|HideQuickSlots _returnvalue_4)
            (bind _returnvalue_5 (Class|InGameHUD|GetPlayerInventoryWidget (Variables|Default|GetInGameHUD)))
            (Class|PlayerInventoryWidget|ShowInventory _returnvalue_5)
            (Class|PlayerInventoryWidget|Update _returnvalue_5 (Variables|Default|GetPlayerInventory))
            (bind _returnvalue_6 (Class|InGameHUD|GetInventoryWidget (Variables|Default|GetInGameHUD)))
            (Class|InventoryWidget|ShowInventory _returnvalue_6)
            (Class|InventoryWidget|Update _returnvalue_6 (Variables|Default|GetChestInventory))
            (if (Utilities|Enum|NotEqual(Enum) (Variables|/Script/GameProject.InputStateMachine|GetActState (Variables|Default|GetPlayerStateMachine)) "UI_CraftInv")
              (Variables|/Script/GameProject.InputStateMachine|SetBeforeUI _playerstatemachine (Variables|/Script/GameProject.InputStateMachine|GetActState _playerstatemachine))
              (Variables|/Script/GameProject.InputStateMachine|SetActState _playerstatemachine "UI_CraftInv")
              (Variables|Default|SetisInvOpen true))))))))

(event EventEndFocus
  (bind _returnvalue (Class|InGameHUD|GetHintWidget (Variables|Default|GetInGameHUD)))
  (Class|HintWidget|HideHint _returnvalue))

(event EventStartFocus
  (bind _ascharacter (Utilities|Casting|CastToCharacter (Pawn|GetControlledPawn (Game|GetPlayerController 0))))
  (Variables|Default|SetPlayerStateMachine (Actor|GetComponentbyClass _ascharacter "/Script/GameProject.InputStateMachine"))
  (bind _asin_game_hud (Utilities|Casting|CastToInGameHUD (HUD|GetHUD (Game|GetPlayerController 0))))
  (bind _output_get (Variables|Default|SetInGameHUD _asin_game_hud))
  (bind _returnvalue (Class|InGameHUD|GetHintWidget _output_get))
  (Class|HintWidget|ShowHint _returnvalue "E"))

(fn ConstructionScript)