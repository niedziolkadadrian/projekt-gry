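; Building placement preview actor that re-evaluates every tick whether the building can be placed, storing the result in CanBePlaced.
; It first compares the player's inventory against BuildResources and BuildResourcesQuantity, constructing an item object per class for each lookup.
; It then requires the OvergroundCollision box to be free of overlapping actors and WorldStatic hits.
; Finally, a "Ground" profile box trace at GroundCollision must hit a Landscape.
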(event EventBeginPlay)

(event Collision|EventActorBeginOverlap
  (params (OtherActor :type Actor%20Object%20Reference)))

(event EventTick
  (params (DeltaSeconds :type Float%20%28single-precision%29))
  (CallFunction|CheckBuildConditions))

(fn ConstructionScript)

(fn CheckBuildConditions
  (bind _overgroundcollision (Variables|Default|GetOvergroundCollision))
  (bind _groundcollision (Variables|Default|GetGroundCollision))
  (bind _returnvalue (Transformation|GetWorldTransform _groundcollision))
  (bind _returnvalue_2 (Transformation|GetWorldTransform _overgroundcollision))
  (bind (_location _rotation) (Math|Transform|BreakTransform _returnvalue))
  (bind (_location_2 _rotation_2) (Math|Transform|BreakTransform _returnvalue_2))
  (bind _returnvalue_3 (Math|Rotator|GetRotationXVector _rotation))
  (bind _returnvalue_4 (Math|Rotator|GetRotationXVector _rotation_2))
  ;[1 1 1] Resources Check
  (bind _asals_anim_man_character (Utilities|Casting|CastToALS_AnimMan_Character (Game|GetPlayerCharacter 0)))
  (Variables|Default|SetPlayer _asals_anim_man_character)
  (bind (_array_element _array_index) (Utilities|Array|ForEachLoopwithBreak (Variables|Default|GetBuildResources) :!label _label)
    (:LoopBody
      (bind _returnvalue_5 (Game|ConstructObjectfromClass _array_element (Variables|Default|GetDefaultSceneRoot)))
      (bind _returnvalue_6 (Class|InventoryComponent|GetItemQuantity (Variables|/Script/GameProject.GameProjectCharacter|GetInventory (Variables|Default|GetPlayer)) _returnvalue_5))
      (if (< _returnvalue_6 (Utilities|Array|Get(acopy) (Variables|Default|GetBuildResourcesQuantity) _array_index))
        (Utilities|FlowControl|Sequence
          (:then_0
            (Variables|Default|SetcanBePlaced false))
          (:then_1
            (goto _label Break)))
        (else
          (Variables|Default|SetcanBePlaced true))))
    (:Completed
      (if (Variables|Default|GetcanBePlaced)
        ;[1 1 1] Overground Collision
        (if (== (Utilities|Array|Length (Collision|GetOverlappingActors (Variables|Default|GetOvergroundCollision) 0 :!class /Script/Engine.PrimitiveComponent)) 0)
          (bind _returnvalue_7 (Class|KismetSystemLibrary|BoxTraceSingleforObjects (- _location_2 _returnvalue_4) (+ _location_2 _returnvalue_4) (Components|Box|GetScaledBoxExtent (Variables|Default|GetOvergroundCollision)) _rotation_2 (Utilities|Array|MakeArray "ObjectTypeQuery1") false 0 "ForOneFrame" true "(R=0.000000,G=1.000000,B=0.000000,A=1.000000)" "(R=1.000000,G=0.000000,B=0.000000,A=1.000000)"))
          (if _returnvalue_7
            (Variables|Default|SetcanBePlaced false)
            (else
              ;[1 1 1] Ground Collision
              (bind _outhit (Class|KismetSystemLibrary|BoxTraceSinglebyProfile (- _location _returnvalue_3) (+ _location _returnvalue_3) (Components|Box|GetScaledBoxExtent (Variables|Default|GetGroundCollision)) _rotation "Ground" false 0 "ForOneFrame" true))
              (Utilities|Casting|CastToLandscape (.HitActor (Collision|BreakHitResult _outhit))
                (:then
                  (Variables|Default|SetcanBePlaced true))
                (:CastFailed
                  (Variables|Default|SetcanBePlaced false)))))
          (else
            (Variables|Default|SetcanBePlaced false)))))))